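; Belt attachment actor from the soldier constructor that shows gloves, a drop bag or a carpet as a physics-driven skeletal mesh.
; The Construction Script picks the mesh from AttachmentType and enables physics simulation on all bodies below the "base" bone, excluding that bone.
; Tick wakes all rigid bodies every frame so the simulated parts do not fall asleep.
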(event EventBeginPlay)

(event Collision|EventActorBeginOverlap
  (params (OtherActor :type Actor%20Object%20Reference)))

(event EventTick
  (params (DeltaSeconds :type Float%20%28single-precision%29))
  (Class|PrimitiveComponent|WakeAllRigidBodies (Variables|Default|GetAttachment)))

(fn ConstructionScript
  (bind _attachment (Variables|Default|GetAttachment))
  (switch Utilities|FlowControl|Switch|SwitchonDT_AttachmentType (Variables|Default|GetAttachmentType)
    (:NewEnumerator0
      (Components|SkinnedMesh|SetSkinnedAssetandUpdate _attachment "/Game/Asset/OutgoingAsset/SoldiersConstructor/Meshes/Attachments/SK_Gloves.SK_Gloves" false))
    (:NewEnumerator1
      (Components|SkinnedMesh|SetSkinnedAssetandUpdate _attachment "/Game/Asset/OutgoingAsset/SoldiersConstructor/Meshes/Attachments/SK_DropBag.SK_DropBag" false))
    (:NewEnumerator2
      (Components|SkinnedMesh|SetSkinnedAssetandUpdate _attachment "/Game/Asset/OutgoingAsset/SoldiersConstructor/Meshes/Attachments/SK_Carpet.SK_Carpet" false)))
  (Class|SkeletalMeshComponent|SetAllBodiesBelowSimulatePhysics (Variables|Default|GetAttachment) (Utilities|Name|MakeLiteralName "base") true false))