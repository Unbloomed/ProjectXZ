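; Rocket projectile for the WeaponKit M92 launcher, using a two-stage launch.
; It first gets a small upward impulse, then after a short delay disables gravity, applies a scaled launch impulse as a velocity change and starts the flying animation and exhaust.
; When destroyed, it spawns a scaled Niagara explosion at its location.
; It also supplies the owning weapon's external bullet color as a material parameter.
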(event Custom|ActivateExhaust
  (Components|Animation|PlayAnimation (Variables|Default|GetProjectileSkelMesh) "/Game/Asset/WeaponKit/Bullets/A_RocketM92_Flying.A_RocketM92_Flying" true)
  (Physics|SetEnableGravity (Variables|Default|GetProjectileSphere) false)
  (Physics|AddImpulse (Variables|Default|GetProjectileSphere) (* (CallFunction|CalculateLaunchImpulse) 3.0) "None" true)
  (Rendering|SetVisibility (Variables|Default|GetExhaustParticles) true false))

(event EventEndPlay
  (params (EndPlayReason :type EEndPlayReason%20Enum :default "Destroyed"))
  (bind _explosionparticlesns (Variables|Default|GetExplosionParticlesNS)
    (:then
      (switch Utilities|FlowControl|Switch|SwitchonEEndPlayReason EndPlayReason
        (:Destroyed
          (bind _returnvalue (Niagara|SpawnSystematLocation _explosionparticlesns (Transformation|GetActorLocation) (Transformation|GetActorRotation)))
          (Effects|Components|ParticleSystem|SetFloatParameter _returnvalue "User.Size" 6.0))))
    (:else)))

(event EventBeginPlay
  (|CallParentFunction)
  (Rendering|SetVisibility (Variables|Default|GetExhaustParticles) false false)
  (Physics|AddImpulse (Variables|Default|GetProjectileSphere) "0, 0,392.000000" "None" false)
  (Utilities|FlowControl|Delay 0.2)
  (CallFunction|ActivateExhaust))

(fn ConstructionScript
  (|CallParentFunction))

(fn GetOwnerMaterialParams
  (params (OwningWeapon :type BP%20Weapon%20Actor%20Base%20WK%20Object%20Reference))
  (return 0 "BulletColor" (Utilities|Struct|BreakFWeaponSettings_WK (Variables|/Game/Asset/WeaponKit/Blueprints/Classes/BP_WeaponActorBase_WK.BP_WeaponActorBase_WK_C|GetSettings OwningWeapon))))